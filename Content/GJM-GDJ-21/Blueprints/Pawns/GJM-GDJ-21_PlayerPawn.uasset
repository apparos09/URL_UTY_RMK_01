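; Player pawn that handles power selection, ball launching and pausing.
; It finds the launcher and UI actors at BeginPlay and stores the power level on the UI.
; Until launch, Tick either oscillates power between zero and max by flipping a direction factor, or follows bracket keys when manual control is on.
; Fire passes that power to the launcher, while P toggles the game mode's pause.
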(event `self.ReceiveBeginPlay`
  ;[1 1 1] Set the Game Mode
  (bind _asgjm_gdj_21_game_mode (cast `/Game/GJM-GDJ-21/Blueprints/GJM-GDJ-21_GameMode` (`GameplayStatics.GetGameMode`))
    (:`then`
      (set `self.gameMode` _asgjm_gdj_21_game_mode))
    (:`CastFailed`
      _))
  ;[1 1 1] Sets the Launcher
  (if (not (`KismetSystemLibrary.IsValid` (`self.Launcher`)))
    (bind _returnvalue (`GameplayStatics.GetActorOfClass` "/Game/GJM-GDJ-21/Blueprints/Sprites/GJM-GDJ-21_Launcher.GJM-GDJ-21_Launcher_C"))
    (set `self.Launcher` _returnvalue))
  ;[1 1 1] Sets the User Interface
  (if (not (`KismetSystemLibrary.IsValid` (`self.UI_Display`)))
    (bind _returnvalue_2 (`GameplayStatics.GetActorOfClass` "/Game/GJM-GDJ-21/Blueprints/GJM-GDJ_21_UI_BP.GJM-GDJ_21_UI_BP_C"))
    (set `self.UI_Display` _returnvalue_2))
  ;[1 1 1] Set Power Direction So That It's Not Zero
  (if (== (`self.PowerAutoFactor`) 0.0)
    (set `self.PowerAutoFactor` 1.0)))

(event `self.ReceiveTick`
  (params (DeltaSeconds :type "Float (single-precision)"))
  (bind _ui_display (`self.UI_Display`))
  (bind _p (`/Game/GJM-GDJ-21/Blueprints/GJM-GDJ-21_GameMode.IsPaused` (`self.gameMode`)))
  (if (not _p)
    ;[1 1 1] Ball Has Not Been Launched Yet
    (if (not (`self.Launched`))
      ;;[0.2762 0.3227 0.7469] Check if Power is Auto Set
      (if (`self.CtrlPower`)
        (if (`self.IncPower`)
          (`/Game/GJM-GDJ-21/Blueprints/GJM-GDJ_21_UI_BP.ChangePowerLevelFixed` _ui_display true true)
          (elif (`self.DecPower`)
            (`/Game/GJM-GDJ-21/Blueprints/GJM-GDJ_21_UI_BP.ChangePowerLevelFixed` _ui_display false true)))
        (else
          (`self.AutoChangePowerLevel`))))))

(event `Key|LeftBracket`
  (params (Key :type "Key Structure"))
  ;[1 1 1] Change Power Level
  (:`Pressed`
    (set `self.DecPower` true))
  (:`Released`
    (set `self.DecPower` false)))

(event `Key|RightBracket`
  (params (Key :type "Key Structure"))
  ;[1 1 1] Change Power Level
  (:`Pressed`
    (set `self.IncPower` true))
  (:`Released`
    (set `self.IncPower` false)))

(event `InputAction|Fire1`
  (params (Key :type "Key Structure"))
  ;[1 1 1] Shoot Ball
  (:`Pressed`
    (bind _p (`/Game/GJM-GDJ-21/Blueprints/GJM-GDJ-21_GameMode.IsPaused` (`self.gameMode`)))
    (if (not _p)
      (bind _launched (`/Game/GJM-GDJ-21/Blueprints/Sprites/GJM-GDJ-21_Launcher.Launch` (`self.Launcher`) (`/Game/GJM-GDJ-21/Blueprints/GJM-GDJ_21_UI_BP.PowerLevel` (`self.UI_Display`))))
      (set `self.Launched` _launched))))

(event `Key|P`
  (params (Key :type "Key Structure"))
  ;[1 1 1] Pause the Game (Don't Disable Input So That It Always Listens for This)
  (:`Pressed`
    (`/Game/GJM-GDJ-21/Blueprints/GJM-GDJ-21_GameMode.ToggleGamePaused` (`self.gameMode`))
    (`KismetSystemLibrary.PrintString` "Pause/Unpaused")))

(fn `AutoChangePowerLevel`
  (bind _ui_display (`self.UI_Display`))
  (bind _ui_display_2 (`self.UI_Display`))
  ;[1 1 1] Change Power Level
  (`/Game/GJM-GDJ-21/Blueprints/GJM-GDJ_21_UI_BP.IncreasePowerLevel` _ui_display (* (`/Game/GJM-GDJ-21/Blueprints/GJM-GDJ_21_UI_BP.PowerLevelInc` _ui_display) (`self.PowerAutoFactor`) (`GameplayStatics.GetWorldDeltaSeconds`)))
  (if (> (`self.PowerAutoFactor`) 0.0)
    ;[1 1 1] Change to Negative
    (if (>= (`/Game/GJM-GDJ-21/Blueprints/GJM-GDJ_21_UI_BP.PowerLevel` _ui_display_2) (`/Game/GJM-GDJ-21/Blueprints/GJM-GDJ_21_UI_BP.PowerLevelMax` _ui_display_2))
      ;[1 1 1] Change Power Direction
      (set `self.PowerAutoFactor` (* (`self.PowerAutoFactor`) -1.0) :!label _label))
    (else
      ;[1 1 1] Change to Positive
      (if (<= (`/Game/GJM-GDJ-21/Blueprints/GJM-GDJ_21_UI_BP.PowerLevel` (`self.UI_Display`)) 0.0)
        (goto _label)
        (else
          _))))
  (return))

(fn `ResetPowerLevel`
  (bind _ui_display (`self.UI_Display`))
  (if (`KismetSystemLibrary.IsValid` _ui_display)
    (`/Game/GJM-GDJ-21/Blueprints/GJM-GDJ_21_UI_BP.ResetPowerLevel` _ui_display)
    (else
      (`KismetSystemLibrary.PrintString` "UI Display Not Set")))
  (return))

(fn `UserConstructionScript`)