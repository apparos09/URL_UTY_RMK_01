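; Player pawn for a GDJAM-21 game jam project that pitches itself each tick based on the mouse cursor position.
; The deprojected cursor location and actor Y feed CreateVectorFromYawPitch as yaw, length and pitch, rather than forming a plain position, to produce the look-at target.
; The Camera counter-rotates by the pitch change to offset the pawn's rotation.
; A debug print shows the cursor's world location every tick.
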(event `self.ReceiveTick`
  (params (DeltaSeconds :type "Float (single-precision)"))
  (bind (_returnvalue_roll _returnvalue_pitch _returnvalue_yaw) (`KismetMathLibrary.BreakRotator` (`self.K2_GetActorRotation`)))
  (bind (_returnvalue_x _returnvalue_y) (`KismetMathLibrary.BreakVector` (`self.K2_GetActorLocation`)))
  (bind _worldlocation (`PlayerController.DeprojectMousePositionToWorld` (`GameplayStatics.GetPlayerController` 0)))
  (bind _pitch (.pitch (`KismetMathLibrary.FindLookAtRotation` (`self.K2_GetActorLocation`) (`KismetMathLibrary.CreateVectorFromYawPitch` (.x _worldlocation) _returnvalue_y (.z _worldlocation)))))
  (bind _output_get (set `self.rotDiff` (- _pitch _returnvalue_pitch)))
  (`self.K2_SetActorRotation` (`KismetMathLibrary.MakeRotator` _returnvalue_roll _pitch _returnvalue_yaw))
  (`SceneComponent.K2_AddWorldRotation` (`self.Camera`) (`KismetMathLibrary.MakeRotator` 0.0 (* _output_get -1.0)) false false)
  (`KismetSystemLibrary.PrintString` (`KismetStringLibrary.Conv_VectorToString` (`PlayerController.DeprojectMousePositionToWorld` (`GameplayStatics.GetPlayerController` 0)))))

(fn `UserConstructionScript`)