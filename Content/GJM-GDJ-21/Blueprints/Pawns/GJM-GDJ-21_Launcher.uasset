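; Launcher pawn that tilts its pitch each Tick to follow the mouse cursor; it contains no firing logic.
; The deprojected cursor X and Z, plus the actor's Y, feed CreateVectorFromYawPitch as yaw, length and pitch, rather than forming a plain position vector.
; A look-at rotation to that vector supplies only pitch, preserving roll and yaw.
; Tick also prints the rotation and mouse world position for debugging.
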(event `self.ReceiveTick`
  (params (DeltaSeconds :type "Float (single-precision)"))
  (bind (_returnvalue_roll _returnvalue_pitch _returnvalue_yaw) (`KismetMathLibrary.BreakRotator` (`self.K2_GetActorRotation`)))
  (bind (_returnvalue_x _returnvalue_y) (`KismetMathLibrary.BreakVector` (`self.K2_GetActorLocation`)))
  (bind _worldlocation (`PlayerController.DeprojectMousePositionToWorld` (`GameplayStatics.GetPlayerController` 0)))
  (bind _returnvalue (`KismetMathLibrary.FindLookAtRotation` (`self.K2_GetActorLocation`) (`KismetMathLibrary.CreateVectorFromYawPitch` (.x _worldlocation) _returnvalue_y (.z _worldlocation))))
  (`self.K2_SetActorRotation` (`KismetMathLibrary.MakeRotator` _returnvalue_roll (.pitch _returnvalue) _returnvalue_yaw))
  (`KismetSystemLibrary.PrintString` (`KismetStringLibrary.Concat_StrStr` "Rot: " (`KismetStringLibrary.Conv_RotatorToString` _returnvalue)))
  (`KismetSystemLibrary.PrintString` (`KismetStringLibrary.Concat_StrStr` "Mouse Wpos:" (`KismetStringLibrary.Conv_VectorToString` (`PlayerController.DeprojectMousePositionToWorld` (`GameplayStatics.GetPlayerController` 0))))))

(fn `UserConstructionScript`)