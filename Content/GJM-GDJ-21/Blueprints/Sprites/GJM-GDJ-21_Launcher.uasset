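; Launcher actor that aims at the mouse cursor and fires the level's GJMGDJ21_Ball.
; BeginPlay finds the ball if none is set, and Tick calls FaceMouse.
; FaceMouse compares the mouse position with the actor's projected screen position, turning the negated look-at yaw into actor pitch.
; Launch fires the ball along the forward vector with base plus added power, only once, guarded by a Launched flag.
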(event `self.ReceiveBeginPlay`
  ;[1 1 1] Sets the Ball
  (if (not (`KismetSystemLibrary.IsValid` (`self.Ball`)))
    (bind _returnvalue (`GameplayStatics.GetActorOfClass` "/Game/GJM-GDJ-21/Blueprints/Sprites/GJM-GDJ-21_Ball.GJM-GDJ-21_Ball_C"))
    (set `self.Ball` _returnvalue)))

(event `self.ReceiveTick`
  (params (DeltaSeconds :type "Float (single-precision)"))
  (`self.FaceMouse`))

(fn `FaceMouse`
  (bind (_returnvalue_roll _returnvalue_pitch _returnvalue_yaw) (`KismetMathLibrary.BreakRotator` (`self.K2_GetActorRotation`)))
  (bind (_locationx _locationy) (`PlayerController.GetMousePosition` (`GameplayStatics.GetPlayerController` 0)))
  ;[1 1 1] Set the Actor's Rotation (Requires Adjustments to be Accurate)
  (`self.K2_SetActorRotation` (struct))
  (`self.K2_SetActorRotation` (`KismetMathLibrary.MakeRotator` _returnvalue_roll (* (.yaw (`KismetMathLibrary.FindLookAtRotation` (`KismetMathLibrary.Vector_Zero`) (- (`KismetMathLibrary.Conv_Vector2DToVector` (`KismetMathLibrary.MakeVector2D` _locationx _locationy)) (`KismetMathLibrary.Conv_Vector2DToVector` (`GameplayStatics.ProjectWorldToScreen` (`GameplayStatics.GetPlayerController` 0) (`self.K2_GetActorLocation`)))))) -1.0) _returnvalue_yaw))
  (return))

(fn `Launch`
  (params (PowerAdd :type "Float (double-precision)"))
  (returns (Launched :type Boolean))
  (if (not (`self.Launched`))
    ;[1 1 1] Launch Ball
    (`/Game/GJM-GDJ-21/Blueprints/Sprites/GJM-GDJ-21_Ball.Launch` (`self.Ball`) (+ (`self.BasePower`) PowerAdd) (`KismetMathLibrary.GetForwardVector` (`self.K2_GetActorRotation`)))
    (set `self.Launched` true))
  (return (`self.Launched`)))

(fn `UserConstructionScript`)