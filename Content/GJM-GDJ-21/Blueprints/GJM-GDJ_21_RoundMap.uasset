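; Round map actor that represents one level layout in a launcher-and-goal ball game, hidden in game from construction.
; BeginPlay caches the game mode and attached actors, then finds the launcher and goal spawn markers among them.
; Activate/Deactivate toggle visibility through the root and collision on each attached actor.
; Activation also resets the player, power level, launcher, ball and goal to the spawns and increments the UI round number.
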(event `self.ReceiveBeginPlay`
  ;[1 1 1] Saves the Game Mode
  (`self.SaveGameMode`)
  ;[1 1 1] Gets All Children
  (set `self.SubActors` (`self.GetAttachedActors` true))
  (`self.SetSpawns`))

(fn `ActivateRoundMap`
  (`self.SetRoundMapActive` true)
  (return))

(fn `DeactivateRoundMap`
  (`self.SetRoundMapActive` false)
  (return))

(fn `Reset Player`
  ;[1 1 1] TODO: share the variable between the player and the launcher.
  (set `/Game/GJM-GDJ-21/Blueprints/Pawns/GJM-GDJ-21_PlayerPawn.Launched` false (`/Game/GJM-GDJ-21/Blueprints/GJM-GDJ-21_GameMode.PlayerPawn` (`self.GDJ-21_GameMode`)))
  (return))

(fn `ResetGoalToSpawn`
  (bind _goal (`/Game/GJM-GDJ-21/Blueprints/GJM-GDJ-21_GameMode.Goal` (`self.GDJ-21_GameMode`)))
  ;[1 1 1] Get Goal
  (if (`KismetSystemLibrary.IsValid` _goal)
    ;[1 1 1] Change the Location
    (`self.K2_SetActorLocation` _goal (`self.K2_GetActorLocation` (`self.GoalSpawn`)) false true)
    (return)
    (else
      (`KismetSystemLibrary.PrintString` "Goal Set Fail")
      (return))))

(fn `ResetLauncherToSpawn`
  (bind _ball (`/Game/GJM-GDJ-21/Blueprints/GJM-GDJ-21_GameMode.Ball` (`self.GDJ-21_GameMode`)))
  ;[1 1 1] Get Launcher
  (if (`KismetSystemLibrary.IsValid` (`/Game/GJM-GDJ-21/Blueprints/GJM-GDJ-21_GameMode.Launcher` (`self.GDJ-21_GameMode`)))
    ;[1 1 1] Reset 'Launched', and 'Power Level'
    (set `/Game/GJM-GDJ-21/Blueprints/Sprites/GJM-GDJ-21_Launcher.Launched` false (`/Game/GJM-GDJ-21/Blueprints/GJM-GDJ-21_GameMode.Launcher` (`self.GDJ-21_GameMode`)))
    (`/Game/GJM-GDJ-21/Blueprints/GJM-GDJ_21_UI_BP.SetPowerLevel` (`/Game/GJM-GDJ-21/Blueprints/GJM-GDJ-21_GameMode.UI_BP` (`self.GDJ-21_GameMode`)) 0.0)
    ;[1 1 1] Change the Location
    (`self.K2_SetActorLocation` (`/Game/GJM-GDJ-21/Blueprints/GJM-GDJ-21_GameMode.Launcher` (`self.GDJ-21_GameMode`)) (`self.K2_GetActorLocation` (`self.LauncherSpawn`)) false true)
    ;[1 1 1] Stops and Positions the Ball (Branch Case Stops Launch Placement Entirely...)
    (`/Game/GJM-GDJ-21/Blueprints/Sprites/GJM-GDJ-21_Ball.Stop` _ball)
    (`self.K2_SetActorLocation` _ball (+ (`self.K2_GetActorLocation` (`self.LauncherSpawn`)) (0.0 0.0 0.0)) false false)
    (return)
    (else
      (`KismetSystemLibrary.PrintString` "Launcher Set Fail")
      (return))))

(fn `SaveGameMode`
  (returns (Success :type Boolean))
  ;[1 1 1] Saves the Game Mode
  (if (not (`KismetSystemLibrary.IsValid` (`self.GDJ-21_GameMode`)))
    (bind _asgjm_gdj_21_game_mode (cast `/Game/GJM-GDJ-21/Blueprints/GJM-GDJ-21_GameMode` (`GameplayStatics.GetGameMode`))
      (:`then`
        (set `self.GDJ-21_GameMode` _asgjm_gdj_21_game_mode))
      (:`CastFailed`
        (return false))))
  (return true))

(fn `SetRoundMapActive`
  (params (Active :type Boolean))
  ;[1 1 1] Hide/Show the Actors
  (`SceneComponent.SetHiddenInGame` (`self.DefaultSceneRoot`) (not Active) true)
  ;[1 1 1] Enable/Disable the SubActors
  (for _array_element (`self.SubActors`)
    (`self.SetActorEnableCollision` _array_element Active))
  (if Active
    ;[1 1 1] Reset the Launcher, Reset the Goal, and Increment the Round Number
    (`self.Reset Player`)
    (`self.ResetLauncherToSpawn`)
    (`self.ResetGoalToSpawn`)
    (`/Game/GJM-GDJ-21/Blueprints/GJM-GDJ_21_UI_BP.IncrementRoundNumber` (`/Game/GJM-GDJ-21/Blueprints/GJM-GDJ-21_GameMode.UI_BP` (`self.GDJ-21_GameMode`))))
  (return))

(fn `SetSpawns`
  ;[1 1 1] Validity Check
  (if (== (`KismetArrayLibrary.Array_Length` (`self.SubActors`)) 0)
    (bind _output_get (set `self.SubActors` (`self.GetAttachedActors` true)))
    (if (== (`KismetArrayLibrary.Array_Length` _output_get) 0)
      (`KismetSystemLibrary.PrintString` "No Sub Actors Found.")
      (return)
      (else
        _)))
  ;[1 1 1] Set Spawns (TODO: add spawns, check for validation, and optimize)
  (for _array_element (`self.SubActors`)
    ;;[1 0.7082 0.2678] Launcher
    (if (not (`KismetSystemLibrary.IsValid` (`self.LauncherSpawn`)))
      (bind _asgjm_gdj_21_launcher_spawn (cast `/Game/GJM-GDJ-21/Blueprints/Sprites/GJM-GDJ-21_LauncherSpawn` _array_element)
        (:`then`
          (set `self.LauncherSpawn` _asgjm_gdj_21_launcher_spawn))
        (:`CastFailed`
          _)))
    (if (`KismetSystemLibrary.IsValid` (`self.GoalSpawn`))
      (break)
      (else
        (bind _asgjm_gdj_21_goal_spawn (cast `/Game/GJM-GDJ-21/Blueprints/Sprites/GJM-GDJ-21_GoalSpawn` _array_element))
        (set `self.GoalSpawn` _asgjm_gdj_21_goal_spawn))))
  (return))

(fn `UserConstructionScript`
  (`SceneComponent.SetHiddenInGame` (`self.DefaultSceneRoot`) true true))