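; Round map Blueprint that groups child actors so a round's map can be switched on or off.
; Construction hides the root and its child components, and BeginPlay caches all child actors.
; Activate and Deactivate call SetRoundMapActive, which sets each child actor's collision to the Active flag.
; The same flag feeds both root NewHidden and PropagateToChildren, so activation hides all child components while deactivation unhides only the root.
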(event `self.ReceiveBeginPlay`
  (set `self.SubActors` (`self.GetAllChildActors` false)))

(fn `ActivateRoundMap`
  (`self.SetRoundMapActive` true)
  (return))

(fn `Deactivate Round Map`
  (`self.SetRoundMapActive` false)
  (return))

(fn `SetRoundMapActive`
  (params (Active :type Boolean))
  ;[1 1 1] Hide/Show the Actors
  (`SceneComponent.SetHiddenInGame` (`self.DefaultSceneRoot`) Active Active)
  ;[1 1 1] Enable/Disable the SubActors
  (for _array_element (`self.SubActors`)
    (`self.SetActorEnableCollision` _array_element Active))
  (return))

(fn `UserConstructionScript`
  (`SceneComponent.SetHiddenInGame` (`self.DefaultSceneRoot`) true true))