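; Game mode for a launcher, ball and goal game that runs a countdown, picks rounds and handles game over.
; BeginPlay caches key actors and round maps, starts the timer, then activates one random round map after deactivating all others.
; Tick counts down and, once launched, checks the ball's X/Z distance from world origin; timeout or out-of-bounds opens the title level.
; Pausing only toggles the countdown, not engine pause.
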(event `self.ReceiveBeginPlay`
  ;[1 1 1] Set the Player Pawn
  (if (not (`KismetSystemLibrary.IsValid` (`self.PlayerPawn`)))
    (bind _returnvalue (`GameplayStatics.GetActorOfClass` "/Game/GJM-GDJ-21/Blueprints/Pawns/GJM-GDJ-21_PlayerPawn.GJM-GDJ-21_PlayerPawn_C"))
    (set `self.PlayerPawn` _returnvalue))
  ;[1 1 1] Sets the Launcher
  (if (not (`KismetSystemLibrary.IsValid` (`self.Launcher`)))
    (bind _returnvalue_2 (`GameplayStatics.GetActorOfClass` "/Game/GJM-GDJ-21/Blueprints/Sprites/GJM-GDJ-21_Launcher.GJM-GDJ-21_Launcher_C"))
    (set `self.Launcher` _returnvalue_2))
  ;[1 1 1] Sets the Ball
  (if (not (`KismetSystemLibrary.IsValid` (`self.Ball`)))
    (bind _returnvalue_3 (`GameplayStatics.GetActorOfClass` "/Game/GJM-GDJ-21/Blueprints/Sprites/GJM-GDJ-21_Ball.GJM-GDJ-21_Ball_C"))
    (set `self.Ball` _returnvalue_3))
  ;[1 1 1] Sets the Goal
  (if (not (`KismetSystemLibrary.IsValid` (`self.Goal`)))
    (bind _returnvalue_4 (`GameplayStatics.GetActorOfClass` "/Game/GJM-GDJ-21/Blueprints/Sprites/GJM-GDJ-21_Goal.GJM-GDJ-21_Goal_C"))
    (set `self.Goal` _returnvalue_4))
  ;[1 1 1] Set the UI
  (if (not (`KismetSystemLibrary.IsValid` (`self.UI_BP`)))
    (bind _returnvalue_5 (`GameplayStatics.GetActorOfClass` "/Game/GJM-GDJ-21/Blueprints/UI/GJM-GDJ_21_UI_BP.GJM-GDJ_21_UI_BP_C"))
    (set `self.UI_BP` _returnvalue_5))
  ;[1 1 1] Set Up Timer
  (set `self.Timer` (`self.TimerStart`))
  (set `self.ActiveTimer` true)
  ;[1 1 1] Set Up Rounds
  (bind _outactors (`GameplayStatics.GetAllActorsOfClass` "/Game/GJM-GDJ-21/Blueprints/GJM-GDJ_21_RoundMap.GJM-GDJ_21_RoundMap_C"))
  (set `self.RoundMaps` _outactors)
  (`self.Next Round`))

(event `self.ReceiveTick`
  (params (DeltaSeconds :type "Float (single-precision)"))
  ;[1 1 1] Updates the Timer
  (`self.UpdateTimer`)
  ;[1 1 1] Checks if the Ball is Out of Bounds Based on the World Origin
  (if (`/Game/GJM-GDJ-21/Blueprints/Sprites/GJM-GDJ-21_Launcher.Launched` (`self.Launcher`))
    (`self.OutOfBoundsCheck`)))

(event `Next Round`
  ;[1 1 1] Goes to the Next Round
  (`self.StartFirstRound`))

(event `self.SetPaused`
  (params (paused :type Boolean))
  ;[1 1 1] Pause Events
  (`self.SetGamePaused` paused))

(event `self.Pause`
  ;[1 1 1] Pause Events
  (`self.SetGamePaused` true))

(event `self.Unpause`
  ;[1 1 1] Pause Events
  (`self.SetGamePaused` false))

(event `self.TogglePaused`
  ;[1 1 1] Pause Events
  (`self.ToggleGamePaused`))

(event `On Game Over`
  ;[1 1 1] On Game Over ITODO: make game over AI)
  (`GameplayStatics.OpenLevel` "TitleWorld"))

(fn `DeactivateAllRounds`
  (if (!= (`KismetArrayLibrary.Array_Length` (`self.RoundMaps`)) 0)
    (for _array_element (`self.RoundMaps`)
      (`/Game/GJM-GDJ-21/Blueprints/GJM-GDJ_21_RoundMap.DeactivateRoundMap` _array_element))
    (return)
    (else
      (return))))

(fn `IsPaused`
  (returns (P :type Boolean))
  (return (`self.Paused`)))

(fn `OutOfBoundsCheck`
  (locals (BoundsDistance :type "Float (double-precision)" :default 3000.0))
  (bind (_returnvalue_x _returnvalue_y _returnvalue_z) (`KismetMathLibrary.BreakVector` (`self.K2_GetActorLocation` (`self.Ball`))))
  ;[1 1 1] Checks the Ball's Distance from the World Origin
  (if (not (<= (`KismetMathLibrary.Distance2D` (0.0 0.0) (`KismetMathLibrary.MakeVector2D` _returnvalue_x _returnvalue_z)) (`local.BoundsDistance`)))
    (`KismetSystemLibrary.PrintString` "Out of Bounds")
    (`self.On Game Over`))
  (return))

(fn `ResetTimer`
  (set `self.ActiveTimer` false)
  (set `self.Timer` (`self.TimerStart`))
  (return))

(fn `SetGamePaused`
  (params (p :type Boolean))
  (bind _output_get (set `self.Paused` p))
  (if _output_get
    (set `self.ActiveTimer` false)
    (else
      (set `self.ActiveTimer` true)))
  (return))

(fn `StartFirstRound`
  ;[1 1 1] Check for Next Rounds
  (if (> (`KismetArrayLibrary.Array_Length` (`self.RoundMaps`)) 0)
    ;[1 1 1] Deactivate Current Round
    (if (`KismetSystemLibrary.IsValid` (`self.CurrentRound`))
      (`/Game/GJM-GDJ-21/Blueprints/GJM-GDJ_21_RoundMap.DeactivateRoundMap` (`self.CurrentRound`)))
    ;[1 1 1] Sets the Current Round and Activates the Round Map
    (bind _output_get (set `self.CurrentRound` (`|GetArrayItem` (`self.RoundMaps`) (`KismetMathLibrary.RandomInteger` (`KismetArrayLibrary.Array_Length` (`self.RoundMaps`))))))
    (`self.DeactivateAllRounds`)
    (`/Game/GJM-GDJ-21/Blueprints/GJM-GDJ_21_RoundMap.ActivateRoundMap` _output_get)
    (return)
    (else
      ;[1 1 1] No New Round, So Game Over
      (`KismetSystemLibrary.PrintString` "There are No Rounds.")
      (`self.On Game Over`)
      (return))))

(fn `ToggleGamePaused`
  (bind _output_get (set `self.Paused` (not (`self.Paused`))))
  (`self.SetPaused` _output_get))

(fn `UpdateTimer`
  (bind _returnvalue (- (`self.Timer`) (`GameplayStatics.GetWorldDeltaSeconds`)))
  ;[1 1 1] Count Down on the Timer
  (if (`self.ActiveTimer`)
    (if (< _returnvalue 0.0)
      (set `self.Timer` 0.0)
      (else
        (set `self.Timer` _returnvalue)))
    ;[1 1 1] Calls Time Over Event if Time is 0
    (if (<= (`self.Timer`) 0.0)
      (`KismetSystemLibrary.PrintString` "Time Over")
      (`self.On Game Over`))
    (return)
    (else
      (return))))

(fn `UserConstructionScript`)