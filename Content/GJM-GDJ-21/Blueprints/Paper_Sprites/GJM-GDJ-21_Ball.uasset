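; Paper2D ball actor that is launched as a physics-simulated sprite and can trigger game over when it comes to rest.
; Launch enables physics and applies a directional impulse, while Stop disables physics and clears velocity, rotation and the idle timer.
; While unpaused, Tick times how long the simulating ball stays still during a running game, calling the GameMode's OnGameOver at the limit.
; Component hits and overlaps play a wall-hit sound.
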(event `self.ReceiveBeginPlay`
  ;[1 1 1] Saves the Game Mode
  (bind _asgjm_gdj_21_game_mode (cast `/Game/GJM-GDJ-21/Blueprints/GJM-GDJ-21_GameMode` (`GameplayStatics.GetGameMode`)))
  (set `self.GameMode` _asgjm_gdj_21_game_mode))

(event `self.ReceiveActorBeginOverlap`
  (params (OtherActor :type "Actor Object Reference")))

(event `self.ReceiveTick`
  (params (DeltaSeconds :type "Float (single-precision)"))
  (bind _gamemode (`self.GameMode`))
  ;[1 1 1] Check if the Ball Has Stopped Moving, If So, Call a Game Over
  (bind _p (`/Game/GJM-GDJ-21/Blueprints/GJM-GDJ-21_GameMode.IsPaused` _gamemode))
  (if (not _p)
    (bind _returnvalue (`PrimitiveComponent.GetPhysicsLinearVelocity` (`self.RenderComponent`) "None"))
    (if (and (== _returnvalue (0.0 0.0 0.0)) (`/Game/GJM-GDJ-21/Blueprints/GJM-GDJ-21_GameMode.Running` _gamemode) (`SceneComponent.IsSimulatingPhysics` (`self.RenderComponent`) "None"))
      ;;[1 1 1] Ball Has Been Still Long Enough, So Game Over
      (bind _output_get (set `self.EarlyEndTimer` (+ (`self.EarlyEndTimer`) DeltaSeconds)))
      (if (>= _output_get (`self.EarlyEndTimerMax`))
        (`/Game/GJM-GDJ-21/Blueprints/GJM-GDJ-21_GameMode.On Game Over` (`self.GameMode`)))
      (else
        (set `self.EarlyEndTimer` 0.0)))))

(event `self.RenderComponent.OnComponentHit`
  (params (HitComponent :type "PrimitiveComponent Object Reference") (OtherActor :type "Actor Object Reference") (OtherComp :type "PrimitiveComponent Object Reference") (NormalImpulse :type "Vector Structure") (Hit :type "HitResult Structure (by ref)"))
  ;[1 1 1] Play Sound if Hit Solid Object
  (`GameplayStatics.PlaySound2D` "/Game/GJM-GDJ-21/Audio/GJM-GDJ-21_WALL_HIT.GJM-GDJ-21_WALL_HIT" 1.0 1.0 0.0 null null :!label _label))

(event `self.RenderComponent.OnComponentBeginOverlap`
  (params (OverlappedComponent :type "PrimitiveComponent Object Reference") (OtherActor :type "Actor Object Reference") (OtherComp :type "PrimitiveComponent Object Reference") (OtherBodyIndex :type Integer) (bFromSweep :type Boolean) (SweepResult :type "HitResult Structure (by ref)"))
  ;[1 1 1] Play Sound if Hit Solid Object
  (goto _label))

(fn `Launch`
  (params (Power :type "Float (double-precision)") (Direction :type "Vector Structure"))
  ;[1 1 1] If the Physics Aren't Applied, Then the Ball Can be Launched
  (if (not (`SceneComponent.IsSimulatingPhysics` (`self.RenderComponent`) "None"))
    ;[1 1 1] Applies Physics to the Sprite
    (`PrimitiveComponent.SetSimulatePhysics` (`self.RenderComponent`) true)
    ;[1 1 1] Applies Force to Launch the Ball
    (`PrimitiveComponent.AddImpulse` (`self.RenderComponent`) (* Direction Power) "None" false))
  ;[1 1 1] Reset Early End Timer
  (set `self.EarlyEndTimer` 0.0)
  (return))

(fn `Stop`
  ;[1 1 1] Stops the Ball from Moving, Resets its Rotation for Removing All Velocity, and Resets the Early Ending Timer
  (`PrimitiveComponent.SetSimulatePhysics` (`self.RenderComponent`) false)
  (`PrimitiveComponent.SetPhysicsLinearVelocity` (`self.RenderComponent`) (0.0 0.0 0.0) false "None")
  (`self.K2_SetActorRotation` (struct))
  (set `self.EarlyEndTimer` 0.0)
  (return))

(fn `UserConstructionScript`)