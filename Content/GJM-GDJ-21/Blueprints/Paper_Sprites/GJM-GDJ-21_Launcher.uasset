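; Paper2D launcher actor that aims in 2D and fires the ball once along its forward vector.
; On unpaused Ticks, the player pawn's CtrlRot flag selects FaceMouse or AutoRotate, which spins at the pawn's RotAutoFactor.
; Both aim in screen space, negating the look-at yaw to set actor pitch.
; Launch passes base plus added power to the Ball, plays a sound and sets Launched to block repeats.
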(event `self.ReceiveBeginPlay`
  ;[1 1 1] Sets the Player
  (if (not (`KismetSystemLibrary.IsValid` (`self.Player`)))
    (bind _returnvalue (`GameplayStatics.GetActorOfClass` "/Game/GJM-GDJ-21/Blueprints/Pawns/GJM-GDJ-21_PlayerPawn.GJM-GDJ-21_PlayerPawn_C"))
    (set `self.Player` _returnvalue))
  ;[1 1 1] Sets the Ball
  (if (not (`KismetSystemLibrary.IsValid` (`self.Ball`)))
    (bind _returnvalue_2 (`GameplayStatics.GetActorOfClass` "/Game/GJM-GDJ-21/Blueprints/Paper_Sprites/GJM-GDJ-21_Ball.GJM-GDJ-21_Ball_C"))
    (set `self.Ball` _returnvalue_2)))

(event `self.ReceiveTick`
  (params (DeltaSeconds :type "Float (single-precision)"))
  ;[1 1 1] Pause Function
  (bind _p (`/Game/GJM-GDJ-21/Blueprints/GJM-GDJ-21_GameMode.IsPaused` (`/Game/GJM-GDJ-21/Blueprints/Pawns/GJM-GDJ-21_PlayerPawn.GameMode` (`self.Player`))))
  (if (not _p)
    ;[1 1 1] Face the Mouse, or Rotate Automatically (Constraints Don't Seem to Do Anything)
    (if (`/Game/GJM-GDJ-21/Blueprints/Pawns/GJM-GDJ-21_PlayerPawn.CtrlRot` (`self.Player`))
      (`PrimitiveComponent.SetConstraintMode` (`self.RenderComponent`) "XZPlane")
      (`self.FaceMouse`)
      (else
        (`PrimitiveComponent.SetConstraintMode` (`self.RenderComponent`) "None")
        (`self.AutoRotate`)))))

(fn `AutoRotate`
  (locals (LookTarget :type "Vector Structure" :default (1.0 0.0 0.0)))
  (bind (_returnvalue_roll _returnvalue_pitch _returnvalue_yaw) (`KismetMathLibrary.BreakRotator` (`self.K2_GetActorRotation`)))
  (bind _returnvalue (`KismetMathLibrary.Conv_Vector2DToVector` (`GameplayStatics.ProjectWorldToScreen` (`GameplayStatics.GetPlayerController` 0) (`self.K2_GetActorLocation`))))
  (bind _returnvalue_2 (+ (`self.AutoRotAmnt`) (* (`/Game/GJM-GDJ-21/Blueprints/Pawns/GJM-GDJ-21_PlayerPawn.RotAutoFactor` (`self.Player`)) (`GameplayStatics.GetWorldDeltaSeconds`))))
  (bind _returnvalue_3 (mod (`KismetMathLibrary.Abs` _returnvalue_2) 360.0))
  ;[1 1 1] Adjust Rotation Amount
  (if (< _returnvalue_2 0.0)
    (set `self.AutoRotAmnt` (* _returnvalue_3 -1.0))
    (else
      (set `self.AutoRotAmnt` _returnvalue_3)))
  ;[1 1 1] Rotate Target, Then Offset it from the Launcher Screen Location and Get the Look At Rotation
  (bind _output_get (set `local.LookTarget` (10.0 0.0 0.0)))
  (bind _output_get_2 (set `local.LookTarget` (+ _returnvalue (`KismetMathLibrary.GreaterGreater_VectorRotator` _output_get (`KismetMathLibrary.MakeRotator` 0.0 0.0 (`self.AutoRotAmnt`))))))
  ;[1 1 1] Sets the Actor Rotation
  (`self.K2_SetActorRotation` (struct))
  (`self.K2_SetActorRotation` (`KismetMathLibrary.MakeRotator` _returnvalue_roll (* (.yaw (`KismetMathLibrary.FindLookAtRotation` _returnvalue _output_get_2)) -1.0) _returnvalue_yaw))
  (return))

(fn `FaceMouse`
  (bind (_returnvalue_roll _returnvalue_pitch _returnvalue_yaw) (`KismetMathLibrary.BreakRotator` (`self.K2_GetActorRotation`)))
  (bind (_locationx _locationy) (`PlayerController.GetMousePosition` (`GameplayStatics.GetPlayerController` 0)))
  ;[1 1 1] Set the Actor's Rotation (Requires Adjustments to be Accurate)
  (`self.K2_SetActorRotation` (struct))
  (`self.K2_SetActorRotation` (`KismetMathLibrary.MakeRotator` _returnvalue_roll (* (.yaw (`KismetMathLibrary.FindLookAtRotation` (`KismetMathLibrary.Vector_Zero`) (- (`KismetMathLibrary.Conv_Vector2DToVector` (`KismetMathLibrary.MakeVector2D` _locationx _locationy)) (`KismetMathLibrary.Conv_Vector2DToVector` (`GameplayStatics.ProjectWorldToScreen` (`GameplayStatics.GetPlayerController` 0) (`self.K2_GetActorLocation`)))))) -1.0) _returnvalue_yaw))
  (return))

(fn `Launch`
  (params (PowerAdd :type "Float (double-precision)"))
  (returns (Launched :type Boolean))
  (if (not (`self.Launched`))
    ;[1 1 1] Launch Ball
    (`/Game/GJM-GDJ-21/Blueprints/Paper_Sprites/GJM-GDJ-21_Ball.Launch` (`self.Ball`) (+ (`self.BasePower`) PowerAdd) (`KismetMathLibrary.GetForwardVector` (`self.K2_GetActorRotation`)))
    (set `self.Launched` true)
    ;[1 1 1] Launch Sound
    (`GameplayStatics.PlaySound2D` "/Game/GJM-GDJ-21/Audio/URL_UTY_RMK01_LAUNCH.URL_UTY_RMK01_LAUNCH" 1.0 1.0 0.0 null null))
  (return (`self.Launched`)))

(fn `UserConstructionScript`)