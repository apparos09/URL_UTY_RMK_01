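; Goal sprite actor that advances the game to a new round when a Ball overlaps its render component.
; NextRound deactivates the game mode's current round map, activates a random entry from its RoundMaps array and flags the game as running.
; The round-switching logic works directly on GJM-GDJ-21_GameMode state, and a TODO marks it to move out of the Goal.
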(event `self.ReceiveBeginPlay`
  ;[1 1 1] Saves the Game Mode
  (if (not (`KismetSystemLibrary.IsValid` (`self.GDJ-21_GameMode`)))
    (cast `/Game/GJM-GDJ-21/Blueprints/GJM-GDJ-21_GameMode` (`GameplayStatics.GetGameMode`))))

(event `self.ReceiveActorBeginOverlap`
  (params (OtherActor :type "Actor Object Reference")))

(event `self.RenderComponent.OnComponentBeginOverlap`
  (params (OverlappedComponent :type "PrimitiveComponent Object Reference") (OtherActor :type "Actor Object Reference") (OtherComp :type "PrimitiveComponent Object Reference") (OtherBodyIndex :type Integer) (bFromSweep :type Boolean) (SweepResult :type "HitResult Structure (by ref)"))
  ;[1 1 1] Did a Ball Hit the Goal?
  (if (`KismetMathLibrary.ClassIsChildOf` (`GameplayStatics.GetObjectClass` OtherActor) "/Game/GJM-GDJ-21/Blueprints/Paper_Sprites/GJM-GDJ-21_Ball.GJM-GDJ-21_Ball_C")
    (`self.NextRound`)
    (`KismetSystemLibrary.PrintString` "Next Round")))

(fn `NextRound`
  (bind _roundmaps (`/Game/GJM-GDJ-21/Blueprints/GJM-GDJ-21_GameMode.RoundMaps` (`self.GDJ-21_GameMode`)))
  (bind _currentround (`/Game/GJM-GDJ-21/Blueprints/GJM-GDJ-21_GameMode.CurrentRound` (`self.GDJ-21_GameMode`)))
  (bind _returnvalue (`KismetArrayLibrary.Array_Length` _roundmaps))
  ;[1 1 1] Get the Game Mode (TODO: take this out of the Goal blueprint)
  (if (not (`KismetSystemLibrary.IsValid` (`self.GDJ-21_GameMode`)))
    (bind _asgjm_gdj_21_game_mode (cast `/Game/GJM-GDJ-21/Blueprints/GJM-GDJ-21_GameMode` (`GameplayStatics.GetGameMode`))
      (:`then`
        (set `self.GDJ-21_GameMode` _asgjm_gdj_21_game_mode))
      (:`CastFailed`
        (return))))
  ;[1 1 1] Check for Available Rounds
  (if (> _returnvalue 0)
    ;[1 1 1] Deactivate the Current Round
    (if (`KismetSystemLibrary.IsValid` _currentround)
      (`/Game/GJM-GDJ-21/Blueprints/GJM-GDJ_21_RoundMap.DeactivateRoundMap` _currentround))
    ;[1 1 1] Activate the New Round
    (bind _output_get (set `/Game/GJM-GDJ-21/Blueprints/GJM-GDJ-21_GameMode.CurrentRound` (`|GetArrayItem` _roundmaps (`KismetMathLibrary.RandomInteger` _returnvalue)) (`self.GDJ-21_GameMode`)))
    (`/Game/GJM-GDJ-21/Blueprints/GJM-GDJ_21_RoundMap.ActivateRoundMap` _output_get)
    ;[1 1 1] Game Running
    (set `/Game/GJM-GDJ-21/Blueprints/GJM-GDJ-21_GameMode.Running` true (`self.GDJ-21_GameMode`))
    (return)
    (else
      (return))))

(fn `UserConstructionScript`)