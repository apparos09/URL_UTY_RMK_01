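; UI manager actor that creates the game's HUD widget and exposes functions to drive its power bar, timer text and round number.
; Power changes are clamped to a maximum and shown as a bar fraction, with fixed-step changes optionally scaled by delta time.
; Each tick it copies the GJM-GDJ-21 game mode's timer to the text while that timer is active, re-fetching the game mode if invalid.
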(event `self.ReceiveBeginPlay`
  ;[1 1 1] Set up the Interface
  (bind _returnvalue (`|CreateWidget` "/Game/GJM-GDJ-21/Blueprints/GJM-GDJ_21_UI_Display.GJM-GDJ_21_UI_Display_C"))
  (bind _output_get (set `self.UI_Var` _returnvalue))
  (`UserWidget.AddToViewport` _output_get 0)
  (`ProgressBar.SetPercent` (`/Game/GJM-GDJ-21/Blueprints/GJM-GDJ_21_UI_Display.PowerBar` (`self.UI_Var`)) 0.0)
  ;[1 1 1] Save the Game Mode
  (bind _asgjm_gdj_21_game_mode (cast `/Game/GJM-GDJ-21/Blueprints/GJM-GDJ-21_GameMode` (`GameplayStatics.GetGameMode`)))
  (set `self.GameMode` _asgjm_gdj_21_game_mode))

(event `self.ReceiveTick`
  (params (DeltaSeconds :type "Float (single-precision)"))
  (`self.UpdateTimerText`))

(fn `ChangePowerLevelFixed`
  (params (Increase :type Boolean) (ApplyDeltaTime :type Boolean))
  (bind _powerlevelinc (`self.PowerLevelInc`))
  (bind _returnvalue (* _powerlevelinc (`GameplayStatics.GetWorldDeltaSeconds`)))
  ;[1 1 1] Increase or Decrease Based on Boolean (Also Accounts for Delta Time)
  (if Increase
    (if ApplyDeltaTime
      (`self.IncreasePowerLevel` _returnvalue)
      (else
        (`self.IncreasePowerLevel` _powerlevelinc)))
    (elif ApplyDeltaTime
      (`self.DecreasePowerLevel` _returnvalue)
      (else
        (`self.DecreasePowerLevel` _powerlevelinc))))
  (return))

(fn `DecreasePowerLevel`
  (params (Dec :type "Float (double-precision)"))
  (`self.SetPowerLevel` (- (`self.PowerLevel`) Dec))
  (return))

(fn `IncreasePowerLevel`
  (params (Inc :type "Float (double-precision)"))
  (`self.SetPowerLevel` (+ Inc (`self.PowerLevel`)))
  (return))

(fn `IncrementRoundNumber`
  (`/Game/GJM-GDJ-21/Blueprints/GJM-GDJ_21_UI_Display.IncrementRoundNumber` (`self.UI_Var`))
  (return))

(fn `ResetPowerLevel`
  (`self.SetPowerLevel` 0.0))

(fn `Set Round Number`
  (params (Number :type Integer))
  (bind _ui_var (`self.UI_Var`))
  ;[1 1 1] Sets the Round Number (TODO: Add Leading Zeroes)
  (if (< Number 0)
    (`/Game/GJM-GDJ-21/Blueprints/GJM-GDJ_21_UI_Display.SetRoundNumber` _ui_var 0)
    (else
      (`/Game/GJM-GDJ-21/Blueprints/GJM-GDJ_21_UI_Display.SetRoundNumber` _ui_var Number)))
  (return))

(fn `SetPowerBarPercent`
  (params (Percent :type "Float (double-precision)"))
  (`ProgressBar.SetPercent` (`/Game/GJM-GDJ-21/Blueprints/GJM-GDJ_21_UI_Display.PowerBar` (`self.UI_Var`)) Percent)
  (return))

(fn `SetPowerLevel`
  (params (NewPower :type "Float (double-precision)"))
  ;[1 1 1] Set Power Level
  (bind _output_get (set `self.PowerLevel` (`KismetMathLibrary.FClamp` NewPower 0.0 (`self.PowerLevelMax`))))
  ;[1 1 1] Set Power Level Percent for Visuals
  (`self.SetPowerBarPercent` (/ _output_get (`self.PowerLevelMax`)))
  (return))

(fn `UpdateTimerText`
  ;[1 1 1] Validity Check
  (`/Engine/EditorBlueprintResources/StandardMacros.IsValid` (`self.GameMode`)
    (:`Is Valid`
      _)
    (:`Is Not Valid`
      (bind _asgjm_gdj_21_game_mode (cast `/Game/GJM-GDJ-21/Blueprints/GJM-GDJ-21_GameMode` (`GameplayStatics.GetGameMode`))
        (:`then`
          (set `self.GameMode` _asgjm_gdj_21_game_mode))
        (:`CastFailed`
          (return)))))
  ;[1 1 1] Convert Time Float to Text (TODO: format time)
  (if (`/Game/GJM-GDJ-21/Blueprints/GJM-GDJ-21_GameMode.ActiveTimer` (`self.GameMode`))
    (`TextBlock.SetText` (`/Game/GJM-GDJ-21/Blueprints/GJM-GDJ_21_UI_Display.TimeText` (`self.UI_Var`)) (`KismetTextLibrary.Conv_DoubleToText` (`/Game/GJM-GDJ-21/Blueprints/GJM-GDJ-21_GameMode.Timer` (`self.GameMode`)) "HalfToEven")))
  (return))

(fn `UserConstructionScript`)